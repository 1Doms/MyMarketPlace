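; Lobby game mode that caps the player count at the online session's connection limit.
; BeginPlay reads that limit from the session settings as the max slot count.
; PostLogin tracks each new controller and, if the GameState PlayerArray exceeds the limit, untracks and kicks it as "Full".
; Every login, kicked or not, then triggers a session update that re-submits the current settings unchanged.
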(event `self.ReceiveBeginPlay`
  (bind _numconnections (`AdvancedSessionsLibrary.GetSessionSettings`)
    (:`OnSuccess`
      (set `self.I_MaxPlayerSlot` _numconnections))))

(event `self.HandleStartingNewPlayer`
  (params (NewPlayer :type "PlayerController Object Reference")))

(event `self.K2_PostLogin`
  (params (NewPlayer :type "PlayerController Object Reference"))
  (set `self.PC_CurrentController` NewPlayer)
  (`KismetArrayLibrary.Array_AddUnique` (`self.PlayersController`) (`self.PC_CurrentController`))
  (if (`self.FC_HasTooMuchPlayer?`)
    (`KismetArrayLibrary.Array_RemoveItem` (`self.PlayersController`) (`self.PC_CurrentController`))
    (`AdvancedSessionsLibrary.KickPlayer` (`self.PC_CurrentController`) "Full")
    (`self.CE_UpdateSession`)
    (else
      (`self.CE_UpdateSession`))))

(event `CE_UpdateSession`
  (bind (_numconnections _numprivateconnections _bislan _bisdedicated _ballowinvites _ballowjoininprogress _bisanticheatenabled _builduniqueid _extrasettings) (`AdvancedSessionsLibrary.GetSessionSettings`)
    (:`OnSuccess`
      (`UpdateSessionCallbackProxyAdvanced.UpdateSession` _extrasettings _numconnections _numprivateconnections _bislan _ballowinvites _ballowjoininprogress true _bisdedicated))))

(fn `FC_HasTooMuchPlayer?`
  (returns (ReturnValue :type Boolean))
  (return (> (`KismetArrayLibrary.Array_Length` (`GameStateBase.PlayerArray` (`GameplayStatics.GetGameState`))) (`self.I_MaxPlayerSlot`))))

(fn `UserConstructionScript`)